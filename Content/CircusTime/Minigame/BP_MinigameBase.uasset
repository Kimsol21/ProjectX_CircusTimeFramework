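; BP_MinigameBase is a base Blueprint for minigames, driving the pre-game flow from info screen through countdown to start.
; OnConstruct caches the CT_PlayerController, which PreProcessGame uses to show the game info widget when a player enters.
; Widget delegates chain the stages: the start button shows the countdown widget, whose end triggers GameStart.
; GameStart removes that widget and only prints a message, while GameEnd is an empty stub.
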(event Custom|StartCountDown
  ;[1 1 1] 카운트다운 시작 시 호출
  (bind _madewidget (Default|UploadUItoScreen (Variables|Default|GetCurrentPlayController) (Variables|Default|GetClass_GameStartWidget)))
  (bind _aswdg_game_start (Utilities|Casting|CastToWDG_GameStart _madewidget))
  (EventDispatchers|AssignCountDownEndDelegate _aswdg_game_start (delegate Custom|GameStart)))

(event Custom|OnConstruct
  (params (PlayerController :type Player%20Controller%20Object%20Reference))
  ;[1 1 1] BeginPlay시 호출
  (bind _asct_player_controller (Utilities|Casting|CastToCT_PlayerController PlayerController))
  (Variables|Default|SetCurrentPlayController _asct_player_controller))

(event Custom|GameStart
  ;[1 1 1] 게임 시작 시 호출
  (Default|RemoveUItoScreen (Variables|Default|GetCurrentPlayController) (stale Custom|StartCountDown _madewidget))
  (Development|PrintText 0 "GameStart"))

(event Custom|PreProcessGame
  ;[1 1 1] 플레이어가 미니게임 입장시 호출
  (bind _madewidget (Default|UploadUItoScreen (Variables|Default|GetCurrentPlayController) (Variables|Default|GetClass_GameInfoWidget)))
  (bind _aswdg_game_info (Utilities|Casting|CastToWDG_GameInfo _madewidget))
  (EventDispatchers|AssignStartButtonClickEvent _aswdg_game_info (delegate Custom|StartCountDown)))

(fn GameEnd)